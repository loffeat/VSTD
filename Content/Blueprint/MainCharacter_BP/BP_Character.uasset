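; Paper2D player character that moves on two axes and carries a weapon sprite aimed at the mouse cursor.
; The Vertical axis event sets FaceDirection, which Tick uses to pick and flip the body flipbook and to swap and offset the weapon sprite.
; Tick also yaws the weapon toward the cursor hit and refreshes TowerData from the Data_Towers "Weapon" row.
; Left mouse only toggles an Attacking flag, set while AttackMode is on.
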(event EventTick
  (params (DeltaSeconds :type Float%20%28single-precision%29))
  (bind _returnvalue (Transformation|GetActorRotation))
  (bind _sprite (Variables|Default|GetSprite))
  (bind _sprite_2 (Variables|Default|GetSprite))
  (bind _papersprite (Variables|Default|GetPaperSprite))
  (bind _papersprite_2 (Variables|Default|GetPaperSprite))
  (Utilities|FlowControl|Sequence
    (:then_0
      ;[1 1 1] FaceDirection, WeaponDirection
      (switch Utilities|FlowControl|Switch|SwitchonE_FaceDirection (Variables|Default|GetFaceDirection)
        (:NewEnumerator0
          (Transformation|SetRelativeRotation _sprite "0, 0, 0" false false)
          (Sprite|SetFlipbook _sprite_2 "/Game/Assets/Character/Player_Up.Player_Up")
          (Rendering|Components|Sprite|SetSprite _papersprite_2 (.top (Variables|Default|GetTowerData)))
          (Transformation|SetRelativeLocation _papersprite "0.000000,0.000000,8.000000" false false))
        (:NewEnumerator1
          (Transformation|SetRelativeRotation _sprite "0, 0, 0" false false)
          (Sprite|SetFlipbook _sprite_2 "/Game/Assets/Character/Player_Down.Player_Down")
          (Rendering|Components|Sprite|SetSprite _papersprite_2 (.down (Variables|Default|GetTowerData)))
          (Transformation|SetRelativeLocation _papersprite "0.000000,0.000000,-4.000000" false false))
        (:NewEnumerator2
          (Transformation|SetRelativeRotation _sprite "0.000000,180.000000,0.000000" false false)
          (Sprite|SetFlipbook _sprite_2 "/Game/Assets/Character/Player_Side.Player_Side")
          (Rendering|Components|Sprite|SetSprite _papersprite_2 (.left (Variables|Default|GetTowerData)))
          (Transformation|SetRelativeLocation _papersprite "-6.000000,0.000000,-3.000000" false false))
        (:NewEnumerator3
          (Transformation|SetRelativeRotation _sprite "0, 0, 0" false false)
          (Sprite|SetFlipbook _sprite_2 "/Game/Assets/Character/Player_Side.Player_Side")
          (Rendering|Components|Sprite|SetSprite _papersprite_2 (.right (Variables|Default|GetTowerData)))
          (Transformation|SetRelativeLocation _papersprite "6.000000,0.000000,-3.000000" false false))
        (:NewEnumerator4
          (Transformation|SetRelativeRotation _sprite "0.000000,180.000000,0.000000" false false)
          (Sprite|SetFlipbook _sprite_2 "/Game/Assets/Character/Player_Up.Player_Up")
          (Rendering|Components|Sprite|SetSprite _papersprite_2 (.topleft (Variables|Default|GetTowerData)))
          (Transformation|SetRelativeLocation _papersprite "-5.000000,0.000000,5.000000" false false))
        (:NewEnumerator5
          (Transformation|SetRelativeRotation _sprite "0, 0, 0" false false)
          (Sprite|SetFlipbook _sprite_2 "/Game/Assets/Character/Player_Up.Player_Up")
          (Rendering|Components|Sprite|SetSprite _papersprite_2 (.topright (Variables|Default|GetTowerData)))
          (Transformation|SetRelativeLocation _papersprite "5.000000,0.000000,5.000000" false false))
        (:NewEnumerator6
          (Transformation|SetRelativeRotation _sprite "0.000000,180.000000,0.000000" false false)
          (Sprite|SetFlipbook _sprite_2 "/Game/Assets/Character/Player_Down.Player_Down")
          (Rendering|Components|Sprite|SetSprite _papersprite_2 (.downleft (Variables|Default|GetTowerData)))
          (Transformation|SetRelativeLocation _papersprite "-4.000000,0.000000,-4.000000" false false))
        (:NewEnumerator7
          (Transformation|SetRelativeRotation _sprite "0, 0, 0" false false)
          (Sprite|SetFlipbook _sprite_2 "/Game/Assets/Character/Player_Down.Player_Down")
          (Rendering|Components|Sprite|SetSprite _papersprite_2 (.downright (Variables|Default|GetTowerData)))
          (Transformation|SetRelativeLocation _papersprite "4.000000,0.000000,-4.000000" false false))))
    (:then_1
      ;[1 1 1] TowerRotation Toward Mouse
      (Transformation|SetWorldRotation (Variables|Default|GetPaperSprite) (Math|Rotator|MakeRotator (.roll _returnvalue) (.pitch _returnvalue) (.yaw (Math|Rotator|FindLookatRotation (Transformation|GetActorLocation) (.Location (Collision|BreakHitResult (.HitResult (Game|Player|GetHitResultUnderCursorbyChannel (Game|GetPlayerController 0) "TraceTypeQuery1" true))))))) false false))
    (:then_2
      (bind _returnvalue_2 (Utilities|GetDataTableRow "/Game/Blueprint/Objects_BP/Data_Towers.Data_Towers" "Weapon")
        (:then
          (Variables|Default|SetTowerData _returnvalue_2))))))

(event Input|AxisEvents|InputAxisHorizontalMoving
  (params (AxisValue :type Float%20%28single-precision%29))
  ;[1 1 1] Find FaceDirection
  (Pawn|Input|AddMovementInput "1.000000,0.000000,0.000000" AxisValue false))

(event Input|AxisEvents|InputAxisVerticalMoving
  (params (AxisValue :type Float%20%28single-precision%29))
  ;[1 1 1] Find FaceDirection
  (Pawn|Input|AddMovementInput "0.000000,1.000000,0.000000" AxisValue false)
  (Math|Float|CompareFloat AxisValue 0.0
    (:>
      (Math|Float|CompareFloat (stale Input|AxisEvents|InputAxisHorizontalMoving AxisValue) 0.0
        (:>
          (Variables|Default|SetFaceDirection "NewEnumerator7"))
        (:==
          (Variables|Default|SetFaceDirection "NewEnumerator1"))
        (:<
          (Variables|Default|SetFaceDirection "NewEnumerator6"))))
    (:==
      (Math|Float|CompareFloat (stale Input|AxisEvents|InputAxisHorizontalMoving AxisValue) 0.0
        (:>
          (Variables|Default|SetFaceDirection "NewEnumerator3"))
        (:==
          (Variables|Default|SetFaceDirection "NewEnumerator8"))
        (:<
          (Variables|Default|SetFaceDirection "NewEnumerator2"))))
    (:<
      (Math|Float|CompareFloat (stale Input|AxisEvents|InputAxisHorizontalMoving AxisValue) 0.0
        (:>
          (Variables|Default|SetFaceDirection "NewEnumerator5"))
        (:==
          (Variables|Default|SetFaceDirection "NewEnumerator0"))
        (:<
          (Variables|Default|SetFaceDirection "NewEnumerator4"))))))

(event Input|MouseEvents|LeftMouseButton
  (params (Key :type Key%20Structure :default "None"))
  ;[1 1 1] AttackSystem
  (:Pressed
    (if (Variables|Default|GetAttackMode?)
      (Variables|Default|SetAttacking? true)))
  (:Released
    (Variables|Default|SetAttacking? false)))

(fn ConstructionScript)
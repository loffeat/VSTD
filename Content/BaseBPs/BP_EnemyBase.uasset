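; BP_EnemyBase is an enemy base Blueprint that drops money and exp pickups through its Die handler.
; BeginPlay binds Die to the VPTDAttribute health-changed delegate.
; Die acts on any non-positive Delta, without checking NewHealth, and spawns randomly offset BP_ItemMoney and BP_ItemExp actors using STDrop counts.
; DestroyActor sits inside the exp loop body, so it runs only when that loop iterates.
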(event Custom|Die
  (params (InstigatorActor :type Actor%20Object%20Reference) (OwningComp :type VPTD%20Attribute%20Component%20Object%20Reference) (NewHealth :type Float%20%28single-precision%29) (Delta :type Float%20%28single-precision%29))
  (bind _returnvalue (Math|Random|RandomIntegerinRange 1 5))
  (bind _returnvalue_2 (Transformation|GetActorLocation))
  (bind _st_drop (Variables|Default|GetST_Drop))
  (if (<= Delta 0.0)
    (Development|PrintString "enemy dead" true true "(R=1.000000,G=0.000000,B=0.315367,A=1.000000)")
    (for _index (range 1 (.moneynum _st_drop))
      (Game|SpawnActorfromClass "/Game/BP_ItemMoney.BP_ItemMoney_C" (Math|Transform|MakeTransform (- _returnvalue_2 (Math|Vector|MakeVector _returnvalue _returnvalue 0.0)) "0, 0, 0" "1.000000,1.000000,1.000000") "Undefined" "MultiplyWithRoot" 0 0))
    (for _index_2 (range 1 (.expnum _st_drop))
      (Game|SpawnActorfromClass "/Game/BP_ItemExp.BP_ItemExp_C" (Math|Transform|MakeTransform (+ (Math|Vector|MakeVector (* _index_2 (Math|Random|RandomIntegerinRange 1 5)) (* _index_2 (Math|Random|RandomIntegerinRange 1 5)) 0.0) _returnvalue_2) "0, 0, 0" "1.000000,1.000000,1.000000") "Undefined" "MultiplyWithRoot" 0 0)
      (Actor|DestroyActor))))

(event EventBeginPlay
  (EventDispatchers|AssignOnHealthChangedDelegated (Variables|Default|GetVPTDAttribute) (delegate Custom|Die)))

(fn ConstructionScript
  (|CallParentFunction))
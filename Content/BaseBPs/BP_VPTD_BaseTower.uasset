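; Base tower actor that periodically fires a test projectile at an enemy within range.
; A looping timer sphere-traces for enemy pawns and records their XY distances.
; A hand-written bubble sort aims to put the nearest first, but its index never advances, so only the first two are compared.
; The projectile spawns yawed toward the first entry; construction fixes the tower's height and roll.
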(event Custom|FindEnemies
  (bind _returnvalue (Transformation|GetActorLocation))
  (bind _returnvalue_2 (Transformation|GetActorLocation))
  (bind _returnvalue_3 (Transformation|GetActorLocation))
  (bind _enemiesdistances (Variables|Default|GetEnemiesDistances))
  (bind _enemiesdistances_2 (Variables|Default|GetEnemiesDistances))
  (bind _returnvalue_4 (Utilities|Array|LastIndex _enemiesdistances_2))
  (bind _returnvalue_5 (- _returnvalue_3 _returnvalue_2))
  (Utilities|FlowControl|Sequence
    (:then_0
      (Utilities|Array|Clear (Variables|Default|GetEnemiesInRange))
      (Utilities|Array|Clear (Variables|Default|GetEnemiesDistances))
      (bind _outhits (Collision|MultiSphereTraceForObjects _returnvalue _returnvalue (Variables|Default|GetRange) (Utilities|Array|MakeArray "ObjectTypeQuery3") false 0 "None"))
      (for _array_element _outhits
        (bind _asbp_enemy_base (Utilities|Casting|CastToBP_EnemyBase (.HitActor (Collision|BreakHitResult _array_element))))
        (Utilities|Array|Add (Variables|Default|GetEnemiesInRange) _asbp_enemy_base)))
    (:then_1
      (for _array_element_2 (Variables|Default|GetEnemiesInRange)
        (Utilities|Array|Add (Variables|Default|GetEnemiesDistances) (Math|Vector|VectorLengthXY (- (Transformation|GetActorLocation _array_element_2) (Transformation|GetActorLocation))))
        (Development|PrintString (Utilities|String|ToString(Float) (Math|Vector|VectorLengthXY (- (Transformation|GetActorLocation _array_element_2) (Transformation|GetActorLocation)))))))
    (:then_2
      ;[1 1 1] 冒泡排序
      (Variables|Default|SetCompareTimes _returnvalue_4)
      (for _index (range 1 _returnvalue_4)
        (Variables|Default|SetArrayIndexes 0)
        (for _index_2 (range 1 (Variables|Default|GetCompareTimes))
          (if (> (Utilities|Array|Get(acopy) _enemiesdistances (Variables|Default|GetArrayIndexes)) (Utilities|Array|Get(acopy) _enemiesdistances (+ (Variables|Default|GetArrayIndexes) 1)))
            (Utilities|FlowControl|Sequence
              (:then_0
                (Utilities|Array|Swap (Variables|Default|GetEnemiesInRange) (Variables|Default|GetArrayIndexes) (+ (Variables|Default|GetArrayIndexes) 1)))
              (:then_1
                (Utilities|Array|Swap (Variables|Default|GetEnemiesDistances) (Variables|Default|GetArrayIndexes) (+ (Variables|Default|GetArrayIndexes) 1))
                (Variables|Default|SetCompareTimes (+ (Variables|Default|GetArrayIndexes) 1) :!label _label)))
            (else
              (goto _label))))
        (Variables|Default|SetCompareTimes (- (Variables|Default|GetCompareTimes) 1))))
    (:then_3
      (Utilities|IsValid (Utilities|Array|Get(acopy) (Variables|Default|GetEnemiesInRange))
        (:Is%20Valid
          (Game|SpawnActorfromClass "/Game/BP_TestProjectile.BP_TestProjectile_C" (Math|Transform|MakeTransform (- (Transformation|GetActorLocation) (* (Math|Vector|Normalize (Math|Vector|MakeVector (.x _returnvalue_5) (.y _returnvalue_5) 0.0)) 1e+01)) (Math|Rotator|MakeRotator 0.0 0.0 (.yaw (Math|Rotator|FindLookatRotation (Transformation|GetActorLocation) (Transformation|GetActorLocation (Utilities|Array|Get(acopy) (Variables|Default|GetEnemiesInRange))))))) "Undefined" "MultiplyWithRoot" 0 0)
          (Development|PrintString "projectile spwan"))))))

(event EventBeginPlay
  (Utilities|Time|SetTimerbyEvent (delegate Custom|FindEnemies) 3.0 true))

(fn ConstructionScript
  (bind _returnvalue (Transformation|GetActorLocation))
  (bind _returnvalue_2 (Transformation|GetActorRotation))
  (Transformation|SetActorLocation (Math|Vector|MakeVector (.x _returnvalue) (.y _returnvalue) 2e+01) false false)
  (Transformation|SetActorRotation (Math|Rotator|MakeRotator -9e+01 (.pitch _returnvalue_2) (.yaw _returnvalue_2))))
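; BP_TestEnemy is a test enemy that closes in on the first player's pawn in periodic jumps.
; On BeginPlay, after calling its parent, it starts a looping timer bound to EnemyMove.
; Each tick of that timer offsets the actor by a fixed fraction of the vector to the player, so steps shrink as it nears.
; Movement has no sweep, so obstacles do not block it.
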(event Custom|EnemyMove
  (Transformation|AddActorWorldOffset (* (- (Transformation|GetActorLocation (Game|Player|GetPlayerPawn 0)) (Transformation|GetActorLocation)) "0.300000,0.300000,0.300000")))

(event EventBeginPlay
  (|CallParentFunction)
  (Utilities|Time|SetTimerbyEvent (delegate Custom|EnemyMove) 2.0 true))

(fn ConstructionScript
  (|CallParentFunction))